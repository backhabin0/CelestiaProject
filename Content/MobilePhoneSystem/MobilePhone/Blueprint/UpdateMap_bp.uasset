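; Trigger actor that changes the map shown in the mobile phone's GPS when a third-person player character enters its box.
; On overlap it casts to BP_ThirdPersonCharacter and reaches the GPS map widget through the MobilePhoneComponent's phone UI, if that UI is valid.
; It then applies its own map image and dimensions to the widget's brush and sets the widget's Maps value from MapRoom.
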(event `self.Box.OnComponentBeginOverlap`
  (params (OverlappedComponent :type "PrimitiveComponent Object Reference") (OtherActor :type "Actor Object Reference") (OtherComp :type "PrimitiveComponent Object Reference") (OtherBodyIndex :type Integer) (bFromSweep :type Boolean) (SweepResult :type "HitResult Structure (by ref)"))
  ;[1 1 1] Update Player Map On Overlap
  (bind _asbp_third_person_character (cast `/Game/ThirdPerson/Blueprints/BP_ThirdPersonCharacter` OtherActor))
  (bind _phoneui (`/Game/MobilePhoneSystem/MobilePhone/Components/MobilePhoneComponent.phoneui` (`/Game/ThirdPerson/Blueprints/BP_ThirdPersonCharacter.MobilePhoneComponent` _asbp_third_person_character)))
  (`/Engine/EditorBlueprintResources/StandardMacros.IsValid` _phoneui
    (:`Is Valid`
      (bind _map (`/Game/MobilePhoneSystem/MobilePhone/Apps/GPS_WB.map` (`/Game/MobilePhoneSystem/MobilePhone/Apps/Phoneui_WB.GPS_WB` _phoneui)))
      (`Image.SetBrush` (`/Game/MobilePhoneSystem/MobilePhone/Apps/Map_WB.mapimage` _map) (make `SlateBrush` "Image" "NoTile" "NoMirror" (`self.mapdimensons`) (struct) (struct :`SpecifiedColor` (struct :`R` 1.0 :`G` 1.0 :`B` 1.0 :`A` 1.0) :`ColorUseRule` "UseColor_Specified") (struct :`CornerRadii` (struct :`W` 1.0) :`Color` (struct :`SpecifiedColor` (struct) :`ColorUseRule` "UseColor_Specified") :`RoundingType` "HalfHeightRadius") (`self.map`)))
      (set `/Game/MobilePhoneSystem/MobilePhone/Apps/Map_WB.Maps` (`self.MapRoom`) _map))))

(fn `UserConstructionScript`)