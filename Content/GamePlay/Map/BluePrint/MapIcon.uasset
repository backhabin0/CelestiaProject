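; MapIcon is a map actor that sends the player into Hamburger_Level when the main character overlaps its Collision component.
; Every Tick it looks up BP_Sky and copies its Date.
; On overlap it compares the character's WorkDate to that Date, but both branches currently open the same level.
; The Canenter variable is unused.
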(event `self.ReceiveTick`
  (params (DeltaSeconds :type "Float (single-precision)"))
  (bind _returnvalue (`GameplayStatics.GetActorOfClass` "/Game/GamePlay/DayNightSystem/BP_Sky.BP_Sky_C"))
  (set `self.date` (`/Game/GamePlay/DayNightSystem/BP_Sky.date` _returnvalue)))

(event `self.collision.OnComponentBeginOverlap`
  (params (OverlappedComponent :type "PrimitiveComponent Object Reference") (OtherActor :type "Actor Object Reference") (OtherComp :type "PrimitiveComponent Object Reference") (OtherBodyIndex :type Integer) (bFromSweep :type Boolean) (SweepResult :type "HitResult Structure (by ref)"))
  (bind _asbp_main_character (cast `/Game/MainCharacter/BP_MainCharacter` OtherActor))
  (if (== (`/Game/MainCharacter/BP_MainCharacter.WorkDate` _asbp_main_character) (`self.date`))
    (`GameplayStatics.OpenLevelBySoftObjectPtr` "/Game/CookingMiniGame/Hamburger_Level.Hamburger_Level")
    (else
      (`GameplayStatics.OpenLevelBySoftObjectPtr` "/Game/CookingMiniGame/Hamburger_Level.Hamburger_Level"))))

(fn `UserConstructionScript`)