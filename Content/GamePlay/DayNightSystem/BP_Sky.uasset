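; BP_Sky is a day-night cycle actor that tracks time of day and date.
; Each tick advances Time by delta seconds divided by TimeDilation, resetting it at 24 and incrementing Date.
; Otherwise, Time sets the sun light's pitch, with the moon light held 180 degrees opposite.
; That same branch creates a Phoneui_WB widget every tick without storing it or adding it to the viewport.
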(event `self.ReceiveTick`
  (params (DeltaSeconds :type "Float (single-precision)"))
  (bind _output_get (set `self.Time` (+ (/ DeltaSeconds (`self.TimeDilation`)) (`self.Time`))))
  (if (>= _output_get 24.0)
    (set `self.date` (+ (`self.date`) 1))
    (set `self.Time` 0.0)
    (else
      (`SceneComponent.K2_SetRelativeRotation` (`self.DirectionalLight`) (`KismetMathLibrary.MakeRotator` 0.0 (* (/ (`self.Time`) 24.0) 360.0)) false false)
      (`SceneComponent.K2_SetRelativeRotation` (`self.DirectionalLight1_Moon`) (`KismetMathLibrary.MakeRotator` 0.0 (+ (* (/ (`self.Time`) 24.0) 360.0) 180.0)) false false)
      (`|CreateWidget` "/Game/MobilePhoneSystem/MobilePhone/Apps/Phoneui_WB.Phoneui_WB_C" null null))))

(fn `UserConstructionScript`)