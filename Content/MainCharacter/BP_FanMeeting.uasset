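; BP_FanMeeting is the player character for the fan meeting, with phone, picture-taking, UI and level-open hotkeys.
; FanMeetingItem, limited to FanMeeting_Level while not grabbing, sets the Food mesh from a DataTable row keyed by item ID, plays a montage, then passes the ID to BP_Hari.
; Money loads from LevelGameInstance on BeginPlay, and AddMoney writes it back along with the inventory map.
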(event `self.ReceiveBeginPlay`
  (set `PlayerController.bEnableClickEvents` true (`GameplayStatics.GetPlayerController` 0))
  (bind _aslevel_game_instance (cast `/Game/MainCharacter/LevelGameInstance` (`GameplayStatics.GetGameInstance`)))
  (set `self.Money` (`/Game/MainCharacter/LevelGameInstance.money` _aslevel_game_instance)))

(event `Key|One`
  (params (Key :type "Key Structure"))
  (:`Pressed`
    (`/Game/MobilePhoneSystem/MobilePhone/Components/MobilePhoneComponent.OpenPhone` (`self.MobilePhoneComponent`))))

(event `Key|Four`
  (params (Key :type "Key Structure"))
  (:`Pressed`
    (`/Game/MobilePhoneSystem/MobilePhone/Components/MobilePhoneComponent.Take Picture` (`self.MobilePhoneComponent`))))

(event `Key|Tab`
  (params (Key :type "Key Structure"))
  (bind _returnvalue (`GameplayStatics.GetPlayerController` 0))
  (:`Pressed`
    (bind _returnvalue_2 (`|CreateWidget` "/Game/MainCharacter/Widget/WB_FanMeetingPlayerUI.WB_FanMeetingPlayerUI_C" null null))
    (`UserWidget.AddToViewport` _returnvalue_2 0)
    (`WidgetBlueprintLibrary.SetInputMode_UIOnlyEx` _returnvalue null)
    (set `PlayerController.bShowMouseCursor` true _returnvalue)))

(event `self.FanMeetingItem`
  (params (ItemID :type Integer))
  (if (not (`self.is grab?`))
    (bind _returnvalue (`GameplayStatics.GetCurrentLevelName` true))
    (if (`KismetStringLibrary.EqualEqual_StrStr` _returnvalue "FanMeeting_Level")
      (bind _returnvalue_2 (`|GetDataTableRow` "/Game/FanMeeting/ShopKeeper/FanMeetingItem.FanMeetingItem" (`KismetStringLibrary.Conv_StringToName` (`KismetStringLibrary.Conv_IntToString` ItemID)))
        (:`then`
          (`StaticMeshComponent.SetStaticMesh` (`self.food`) (`.StaticMesh_14_1442AE7F47F2CFEE861153B08EB09BF6` (break `/Game/FanMeeting/ShopKeeper/FanMeetingSturcture` _returnvalue_2)))
          (set `self.grab staticmesh` (`.StaticMesh_14_1442AE7F47F2CFEE861153B08EB09BF6` (break `/Game/FanMeeting/ShopKeeper/FanMeetingSturcture` _returnvalue_2)))
          (`|PlayMontage` (`self.Mesh`) "/Game/MainCharacter/FanMeetingMontage.FanMeetingMontage"
            (:`OnCompleted`
              (bind _returnvalue_3 (`GameplayStatics.GetActorOfClass` "/Game/MetaHumans/Hari/BP_Hari.BP_Hari_C"))
              (message `/Game/FanMeeting/FanMeetingItemInterface.GetItem` _returnvalue_3 ItemID)))))
      (else
        (`KismetSystemLibrary.PrintString` "팬미팅 맵아님")))))

(event `Key|F`
  (params (Key :type "Key Structure"))
  (:`Pressed`
    (`GameplayStatics.OpenLevel` "FanMeeting_Level")))

(fn `AddMoney`
  (params (Addmoney :type Integer))
  (bind _output_get (set `self.Money` (+ (`self.Money`) Addmoney)))
  (bind _aslevel_game_instance (cast `/Game/MainCharacter/LevelGameInstance` (`GameplayStatics.GetGameInstance`)))
  (set `/Game/MainCharacter/LevelGameInstance.money` _output_get _aslevel_game_instance)
  (set `/Game/MainCharacter/LevelGameInstance.inventorymap` (`/Game/MainCharacter/InventoryComponent.InventoryMap` (`self.InventoryComponent`)) _aslevel_game_instance))

(fn `SpendMoney`
  (params (Money :type Integer))
  (returns (remainingmoney :type Integer))
  (set `self.Money` (- (`self.Money`) Money))
  (return 0))

(fn `UserConstructionScript`)