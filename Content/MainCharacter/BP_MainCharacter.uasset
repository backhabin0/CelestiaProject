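; BP_MainCharacter is the player character, handling money, a mobile phone, fan-meeting items and food grabbing.
; Keys drive the phone component's phone, camera and photo features, or open the fan-meeting UI.
; In FanMeeting_Level, item IDs select data-table meshes, play a montage, then notify BP_Hari; grabbed food attaches to a socket, and clicking spawns a copy under the cursor.
; Money loads from LevelGameInstance, and AddMoney writes it back with the inventory map.
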(event `self.ReceiveBeginPlay`
  (set `PlayerController.bEnableClickEvents` true (`GameplayStatics.GetPlayerController` 0))
  (bind _aslevel_game_instance (cast `/Game/MainCharacter/LevelGameInstance` (`GameplayStatics.GetGameInstance`)))
  (set `self.Money` (`/Game/MainCharacter/LevelGameInstance.money` _aslevel_game_instance)))

(event `Key|One`
  (params (Key :type "Key Structure"))
  (:`Pressed`
    (`/Game/MobilePhoneSystem/MobilePhone/Components/MobilePhoneComponent.OpenPhone` (`self.MobilePhoneComponent`))
    (set `PlayerController.bShowMouseCursor` true (`GameplayStatics.GetPlayerController` 0))))

(event `Key|Two`
  (params (Key :type "Key Structure"))
  (:`Pressed`
    (`/Game/MobilePhoneSystem/MobilePhone/Components/MobilePhoneComponent.Open Camera First Person` (`self.MobilePhoneComponent`) (`self.pictureCamera`) (`self.pictureCamera`) self)
    (set `PlayerController.bShowMouseCursor` true (`GameplayStatics.GetPlayerController` 0))))

(event `Key|Four`
  (params (Key :type "Key Structure"))
  ;[1 1 1] Take Picture
  (:`Pressed`
    (`/Game/MobilePhoneSystem/MobilePhone/Components/MobilePhoneComponent.Take Picture` (`self.MobilePhoneComponent`))))

(event `Key|Tab`
  (params (Key :type "Key Structure"))
  (bind _returnvalue (`GameplayStatics.GetPlayerController` 0))
  (:`Pressed`
    (bind _returnvalue_2 (`|CreateWidget` "/Game/MainCharacter/Widget/WB_FanMeetingPlayerUI.WB_FanMeetingPlayerUI_C" null null))
    (`UserWidget.AddToViewport` _returnvalue_2 0)
    (`WidgetBlueprintLibrary.SetInputMode_UIOnlyEx` _returnvalue null)
    (set `PlayerController.bShowMouseCursor` true _returnvalue)))

(event `/Game/MainCharacter/interat/FanmeetingInteract.FanMeetingItem`
  (params (ItemID :type Integer))
  (if (not (`self.is grab?`))
    (bind _returnvalue (`GameplayStatics.GetCurrentLevelName` true))
    (if (`KismetStringLibrary.EqualEqual_StrStr` _returnvalue "FanMeeting_Level")
      (bind _returnvalue_2 (`|GetDataTableRow` "/Game/FanMeeting/ShopKeeper/FanMeetingItem.FanMeetingItem" (`KismetStringLibrary.Conv_StringToName` (`KismetStringLibrary.Conv_IntToString` ItemID)))
        (:`then`
          (`StaticMeshComponent.SetStaticMesh` (`self.food`) (`.StaticMesh_14_1442AE7F47F2CFEE861153B08EB09BF6` (break `/Game/FanMeeting/ShopKeeper/FanMeetingSturcture` _returnvalue_2)))
          (set `self.grab staticmesh` (`.StaticMesh_14_1442AE7F47F2CFEE861153B08EB09BF6` (break `/Game/FanMeeting/ShopKeeper/FanMeetingSturcture` _returnvalue_2)))
          (`|PlayMontage` (`self.Mesh`) "/Game/MainCharacter/FanMeetingMontage.FanMeetingMontage"
            (:`OnCompleted`
              (bind _returnvalue_3 (`GameplayStatics.GetActorOfClass` "/Game/MetaHumans/Hari/BP_Hari.BP_Hari_C"))
              (message `/Game/FanMeeting/FanMeetingItemInterface.GetItem` _returnvalue_3 ItemID)))))
      (else
        (`KismetSystemLibrary.PrintString` "팬미팅 맵아님")))))

(event `/Game/CookingMiniGame/GamePlay/I_FoodGrab.grabFood`
  (params (Socketname :type Name) (Actor :type "Actor Object Reference"))
  (`|PlayMontage` (`self.Mesh`) "/Game/MainCharacter/CookingMontage.CookingMontage" 1.0 0.0 "grabstart"
    (:`OnCompleted`
      (`/Engine/EditorBlueprintResources/StandardMacros.IsValid` Actor
        (:`Is Valid`
          (set `self.GrabActor` Actor)
          (bind _returnvalue (`self.K2_AttachToComponent` Actor (`self.Mesh`) Socketname "SnapToTarget" "SnapToTarget" "SnapToTarget" true))
          (if _returnvalue
            (`KismetSystemLibrary.Delay` 1.0)
            (set `self.is grab?` true)))))))

(event `Key|LeftMouseButton`
  (params (Key :type "Key Structure"))
  (bind _grabactor (`self.GrabActor`))
  (:`Pressed`
    (if (`self.is grab?`)
      (`/Engine/EditorBlueprintResources/StandardMacros.IsValid` _grabactor
        (:`Is Valid`
          (message `/Game/CookingMiniGame/GamePlay/Food/FrenchFry/Interaction/I_LeftFood.FoodLeft` _grabactor)
          (`|SpawnActorFromClass` (`GameplayStatics.GetObjectClass` _grabactor) (`KismetMathLibrary.Conv_VectorToTransform` (`.ImpactPoint` (`GameplayStatics.BreakHitResult` (`PlayerController.GetHitResultUnderCursorByChannel` (`GameplayStatics.GetPlayerController` 0) "TraceTypeQuery1" true)))) "Undefined" "MultiplyWithRoot" null null)
          (`self.K2_DetachFromActor` (`self.GrabActor`) "KeepRelative" "KeepRelative" "KeepRelative")
          (set `self.is grab?` false))))))

(fn `AddMoney`
  (params (Addmoney :type Integer))
  (bind _output_get (set `self.Money` (+ (`self.Money`) Addmoney)))
  (bind _aslevel_game_instance (cast `/Game/MainCharacter/LevelGameInstance` (`GameplayStatics.GetGameInstance`)))
  (set `/Game/MainCharacter/LevelGameInstance.money` _output_get _aslevel_game_instance)
  (set `/Game/MainCharacter/LevelGameInstance.inventorymap` (`/Game/MainCharacter/InventoryComponent.InventoryMap` (`self.InventoryComponent`)) _aslevel_game_instance))

(fn `SpendMoney`
  (params (Money :type Integer))
  (returns (remainingmoney :type Integer))
  (set `self.Money` (- (`self.Money`) Money))
  (return 0))

(fn `UserConstructionScript`)