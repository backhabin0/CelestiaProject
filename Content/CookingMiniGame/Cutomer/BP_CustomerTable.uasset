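; Customer table actor for the cooking minigame that orders a random food and pays the player when it is delivered.
; BeginPlay picks one of three foods from parallel arrays and shows its name on a text render.
; The box overlap identifies Coke, hamburger or fry potato actors through a cast chain and compares the name to the order.
; A match adds food-specific money to the main character, then destroys the table after a short delay.
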(event `self.ReceiveTick`
  (params (DeltaSeconds :type "Float (single-precision)")))

(event `self.ReceiveBeginPlay`
  (bind _random_int1 (`self.random int1`))
  (bind _asbp_main_character (cast `/Game/MainCharacter/BP_MainCharacter` (`GameplayStatics.GetPlayerCharacter` 0)))
  (set `self.As BP Main Character` _asbp_main_character)
  (set `self.random int1` (`KismetMathLibrary.RandomIntegerInRange` 0 2))
  (set `self.wantFood` (`|GetArrayItem` (`self.WantFoodArray`) _random_int1))
  (bind _output_get (set `self.wantFoodName` (`|GetArrayItem` (`self.WantFoodText`) _random_int1)))
  (`TextRenderComponent.K2_SetText` (`self.TextRender`) _output_get))

(event `self.Box.OnComponentBeginOverlap`
  (params (OverlappedComponent :type "PrimitiveComponent Object Reference") (OtherActor :type "Actor Object Reference") (OtherComp :type "PrimitiveComponent Object Reference") (OtherBodyIndex :type Integer) (bFromSweep :type Boolean) (SweepResult :type "HitResult Structure (by ref)"))
  (cast `/Game/CookingMiniGame/GamePlay/Food/Cola/BP_Coke` OtherActor
    (:`then`
      (bind _output_get (set `self.GetFood` "coke"))
      (if (`KismetTextLibrary.EqualEqual_TextText` _output_get (`self.wantFoodName`))
        (`/Game/MainCharacter/BP_MainCharacter.AddMoney` (`self.As BP Main Character`) 2000)
        (`KismetSystemLibrary.Delay` 2.0)
        (`self.K2_DestroyActor`)))
    (:`CastFailed`
      (cast `/Game/CookingMiniGame/GamePlay/Food/Hamberger/BP_HamBarger` OtherActor
        (:`then`
          (bind _output_get_2 (set `self.GetFood` "HamBarger"))
          (if (`KismetTextLibrary.EqualEqual_TextText` _output_get_2 (`self.wantFoodName`))
            (`/Game/MainCharacter/BP_MainCharacter.AddMoney` (`self.As BP Main Character`) 5000)
            (`KismetSystemLibrary.Delay` 2.0)
            (`self.K2_DestroyActor`)))
        (:`CastFailed`
          (cast `/Game/CookingMiniGame/GamePlay/Food/FrenchFry/Food/BP_FryPotato` OtherActor)
          (bind _output_get_3 (set `self.GetFood` "FryPotato"))
          (if (`KismetTextLibrary.EqualEqual_TextText` _output_get_3 (`self.wantFoodName`))
            (`/Game/MainCharacter/BP_MainCharacter.AddMoney` (`self.As BP Main Character`) 4000)
            (`KismetSystemLibrary.Delay` 2.0)
            (`self.K2_DestroyActor`)))))))

(fn `UserConstructionScript`)