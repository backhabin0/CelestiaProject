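; BP_Force is a clickable actor in the cooking minigame that opens the Force widget when selected.
; Its Force component shows a highlight overlay material while the cursor hovers over it and clears it when the cursor leaves.
; On click, the player camera blends to this actor, and after a delay matching the blend the WB_Force widget is added to the viewport.
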(event `self.Force.OnBeginCursorOver`
  (params (TouchedComponent :type "PrimitiveComponent Object Reference"))
  (`MeshComponent.SetOverlayMaterial` (`self.Force`) "/Game/CookingMiniGame/GamePlay/Material/M_Highlight.M_Highlight"))

(event `self.Force.OnEndCursorOver`
  (params (TouchedComponent :type "PrimitiveComponent Object Reference"))
  (`MeshComponent.SetOverlayMaterial` (`self.Force`) null))

(event `self.Force.OnClicked`
  (params (TouchedComponent :type "PrimitiveComponent Object Reference") (ButtonPressed :type "Key Structure"))
  (`PlayerController.SetViewTargetWithBlend` (`GameplayStatics.GetPlayerController` 0) self 2.0 "VTBlend_Linear" 0.0 false)
  (bind _returnvalue (`|CreateWidget` "/Game/CookingMiniGame/Force/WB_Force.WB_Force_C"))
  (`KismetSystemLibrary.Delay` 2.0)
  (`UserWidget.AddToViewport` _returnvalue 0))

(fn `UserConstructionScript`)