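; BP_BreadBottom is the bottom bun actor in the cooking minigame's hamburger assembly.
; Hovering the cursor over its mesh applies a highlight overlay material, using mouse-over events it enables on the player controller at BeginPlay.
; When its capsule overlaps a BP_Patty, it flags that patty's BreadButtomPatty, spawns a BP_HamBarger at the mesh location and destroys itself.
; It also caches the player's BP_MainCharacter at startup.
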(event `self.ReceiveBeginPlay`
  (set `PlayerController.bEnableMouseOverEvents` true (`GameplayStatics.GetPlayerController` 0))
  (bind _asbp_main_character (cast `/Game/MainCharacter/BP_MainCharacter` (`GameplayStatics.GetPlayerCharacter` 0)))
  (set `self.As BP Main Character` _asbp_main_character))

(event `self.StaticMesh.OnBeginCursorOver`
  (params (TouchedComponent :type "PrimitiveComponent Object Reference"))
  (`MeshComponent.SetOverlayMaterial` (`self.StaticMesh`) "/Game/CookingMiniGame/GamePlay/Material/M_Highlight.M_Highlight"))

(event `self.StaticMesh.OnEndCursorOver`
  (params (TouchedComponent :type "PrimitiveComponent Object Reference"))
  (`MeshComponent.SetOverlayMaterial` (`self.StaticMesh`) null))

(event `self.Capsule.OnComponentBeginOverlap`
  (params (OverlappedComponent :type "PrimitiveComponent Object Reference") (OtherActor :type "Actor Object Reference") (OtherComp :type "PrimitiveComponent Object Reference") (OtherBodyIndex :type Integer) (bFromSweep :type Boolean) (SweepResult :type "HitResult Structure (by ref)"))
  (bind _asbp_patty (cast `/Game/CookingMiniGame/GamePlay/Food/Hamberger/BP_Patty` OtherActor))
  (set `/Game/CookingMiniGame/GamePlay/Food/Hamberger/BP_Patty.breadButtomPatty` true _asbp_patty)
  (`|SpawnActorFromClass` "/Game/CookingMiniGame/GamePlay/Food/Hamberger/BP_HamBarger.BP_HamBarger_C" (`KismetMathLibrary.MakeTransform` (`SceneComponent.K2_GetComponentLocation` (`self.StaticMesh`))) "Undefined" "MultiplyWithRoot" null null)
  (`self.K2_DestroyActor`))

(fn `UserConstructionScript`)