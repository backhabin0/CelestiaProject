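; Clickable bread station in the cooking minigame that turns held hamburger meat into a burger item.
; The Bread mesh enables mouse-over events on the player controller and shows a highlight overlay while hovered.
; On click, if the main character's grabbed mesh is the hamburger meat, it hides the bread and spawns BP_Ham at its Scene transform.
; The bread reappears after a short delay, and the character's held mesh is left unchanged here.
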(event `self.ReceiveBeginPlay`
  (set `PlayerController.bEnableMouseOverEvents` true (`GameplayStatics.GetPlayerController` 0)))

(event `self.bread.OnBeginCursorOver`
  (params (TouchedComponent :type "PrimitiveComponent Object Reference"))
  (`MeshComponent.SetOverlayMaterial` (`self.bread`) "/Game/CookingMiniGame/GamePlay/Material/M_Highlight.M_Highlight"))

(event `self.bread.OnEndCursorOver`
  (params (TouchedComponent :type "PrimitiveComponent Object Reference"))
  (`MeshComponent.SetOverlayMaterial` (`self.bread`) null))

(event `self.bread.OnClicked`
  (params (TouchedComponent :type "PrimitiveComponent Object Reference") (ButtonPressed :type "Key Structure"))
  (bind _asbp_main_character (cast `/Game/MainCharacter/BP_MainCharacter` (`GameplayStatics.GetPlayerCharacter` 0)))
  (if (== (`/Game/MainCharacter/BP_MainCharacter.grab staticmesh` _asbp_main_character) "/Game/CookingMiniGame/Food/StaticMesh/NotCooked/SM_hambargerMeat.SM_hambargerMeat")
    (`SceneComponent.SetHiddenInGame` (`self.bread`) true false)
    (`|SpawnActorFromClass` "/Game/CookingMiniGame/GamePlay/Food/Hamberger/BP_Ham.BP_Ham_C" (`SceneComponent.K2_GetComponentToWorld` (`self.Scene`)) "Undefined" "MultiplyWithRoot" null null)
    (`KismetSystemLibrary.Delay` 2.0)
    (`SceneComponent.SetHiddenInGame` (`self.bread`) false false)))

(fn `UserConstructionScript`)