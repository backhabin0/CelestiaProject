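; BP_Grill is the grill in the cooking minigame's hamburger station, timing a raw patty.
; A box overlap flags the patty, stores its location and sets a three-second count.
; Clicking the cylinder starts a Tick-driven countdown shown on a text render.
; CustomEvent_1, not called here, destroys the patty, first spawning BP_FryPotato at its location if the count is between zero and one.
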(event `self.ReceiveTick`
  (params (DeltaSeconds :type "Float (single-precision)"))
  (if (`self.isButtonClick?`)
    (`self.countdown`)))

(event `self.StaticMeshComponent.OnClicked`
  (params (TouchedComponent :type "PrimitiveComponent Object Reference") (ButtonPressed :type "Key Structure")))

(event `self.Box.OnComponentBeginOverlap`
  (params (OverlappedComponent :type "PrimitiveComponent Object Reference") (OtherActor :type "Actor Object Reference") (OtherComp :type "PrimitiveComponent Object Reference") (OtherBodyIndex :type Integer) (bFromSweep :type Boolean) (SweepResult :type "HitResult Structure (by ref)"))
  (bind _asbp_hamberger_pattyraw (cast `/Game/CookingMiniGame/GamePlay/Food/Hamberger/BP_HambergerPattyraw` OtherActor))
  (set `self.is patty?` true)
  (set `/Game/CookingMiniGame/GamePlay/Food/Hamberger/BP_HambergerPattyraw.is in grill?` true _asbp_hamberger_pattyraw)
  (bind _output_get (set `self.As BP Hamberger Pattyraw` _asbp_hamberger_pattyraw))
  (set `self.count` 3.0)
  (set `self.H` (`SceneComponent.K2_GetComponentLocation` (`/Game/CookingMiniGame/GamePlay/Food/Hamberger/BP_HambergerPattyraw.StaticMesh` _output_get))))

(event `self.Cylinder.OnClicked`
  (params (TouchedComponent :type "PrimitiveComponent Object Reference") (ButtonPressed :type "Key Structure"))
  (if (`self.is patty?`)
    (set `self.isButtonClick?` true)))

(event `countdown`
  (bind _output_get (set `self.count` (`KismetMathLibrary.FClamp` (- (`self.count`) (`GameplayStatics.GetWorldDeltaSeconds`)) -3.0 (`self.count`))))
  (`TextRenderComponent.K2_SetText` (`self.TextRender`) (`KismetTextLibrary.Conv_StringToText` (`KismetStringLibrary.TimeSecondsToString` _output_get))))

(event `CustomEvent_1`
  (if (< (`self.count`) 0.0)
    (`self.K2_DestroyActor` (`self.As BP Hamberger Pattyraw`))
    (elif (< (`self.count`) 1.0)
      (`|SpawnActorFromClass` "/Game/CookingMiniGame/GamePlay/Food/FrenchFry/Food/BP_FryPotato.BP_FryPotato_C" (`KismetMathLibrary.Conv_VectorToTransform` (`self.H`)) "Undefined" "MultiplyWithRoot" null null)
      (`self.K2_DestroyActor` (`self.As BP Hamberger Pattyraw`)))))

(fn `UserConstructionScript`)