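; BP_StartPotato is the clickable raw potato that begins the french fry step of the cooking minigame.
; Hovering the mesh shows a highlight overlay, with mouse-over events enabled on BeginPlay, which also caches the main character and the fry machine.
; A click sends a slice message to the fry machine if the potato is in it, otherwise has the character grab it at a socket and disables its collision.
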(event `self.ReceiveBeginPlay`
  (set `PlayerController.bEnableMouseOverEvents` true (`GameplayStatics.GetPlayerController` 0))
  (bind _asbp_main_character (cast `/Game/MainCharacter/BP_MainCharacter` (`GameplayStatics.GetPlayerCharacter` 0)))
  (set `self.As BP Main Character` _asbp_main_character)
  (bind _returnvalue (`GameplayStatics.GetActorOfClass` "/Game/CookingMiniGame/GamePlay/Food/FrenchFry/Food/BP_FryMachine.BP_FryMachine_C"))
  (set `self.FryMachine` _returnvalue))

(event `self.StaticMesh.OnBeginCursorOver`
  (params (TouchedComponent :type "PrimitiveComponent Object Reference"))
  (`MeshComponent.SetOverlayMaterial` (`self.StaticMesh`) "/Game/CookingMiniGame/GamePlay/Material/M_Highlight.M_Highlight"))

(event `self.StaticMesh.OnEndCursorOver`
  (params (TouchedComponent :type "PrimitiveComponent Object Reference"))
  (`MeshComponent.SetOverlayMaterial` (`self.StaticMesh`) null))

(event `self.StaticMesh.OnClicked`
  (params (TouchedComponent :type "PrimitiveComponent Object Reference") (ButtonPressed :type "Key Structure"))
  (if (`self.is in fryMachine?`)
    (message `/Game/CookingMiniGame/GamePlay/Food/FrenchFry/Food/I_SlicePotatoFryMachine.ClickSlicePotato` (`self.FryMachine`))
    (else
      (message `/Game/CookingMiniGame/GamePlay/I_FoodGrab.grabFood` (`self.As BP Main Character`) "PotatoSocket" self)
      (`PrimitiveComponent.SetCollisionEnabled` (`self.StaticMesh`) "NoCollision"))))

(fn `UserConstructionScript`)