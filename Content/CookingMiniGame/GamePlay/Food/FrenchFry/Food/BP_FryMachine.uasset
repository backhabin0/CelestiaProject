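; Fry machine actor for the cooking minigame that turns sliced potato into fried potato.
; Mesh overlap plays a frying sound, flags and stores any BP_SlicePotato, and starts a Tick-driven countdown shown on a TextRender.
; ClickSlicePotato swaps the slice for BP_FryPotato only within the countdown's last second.
; The timer resets only at exactly zero, otherwise running negative to a clamp.
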(event `self.ReceiveTick`
  (params (DeltaSeconds :type "Float (single-precision)"))
  (if (`self.is potato?`)
    (`self.countdown`)))

(event `self.StaticMesh.OnComponentBeginOverlap`
  (params (OverlappedComponent :type "PrimitiveComponent Object Reference") (OtherActor :type "Actor Object Reference") (OtherComp :type "PrimitiveComponent Object Reference") (OtherBodyIndex :type Integer) (bFromSweep :type Boolean) (SweepResult :type "HitResult Structure (by ref)"))
  (`GameplayStatics.PlaySoundAtLocation` "/Game/CookingMiniGame/GamePlay/sound/frying_food.frying_food" (`SceneComponent.K2_GetComponentLocation` (`self.StaticMesh`)) (struct) 1.0 1.0 0.0 null null null null)
  (bind _asbp_slice_potato (cast `/Game/CookingMiniGame/GamePlay/Food/FrenchFry/Food/BP_SlicePotato` OtherActor))
  (set `self.is potato?` true)
  (set `/Game/CookingMiniGame/GamePlay/Food/FrenchFry/Food/BP_SlicePotato.is in fryMachine?` true _asbp_slice_potato)
  (set `self.As BP Slice Potato` _asbp_slice_potato))

(event `countdown`
  (bind _output_get (set `self.count` (`KismetMathLibrary.FClamp` (- (`self.count`) (`GameplayStatics.GetWorldDeltaSeconds`)) -3.0 (`self.count`))))
  (`TextRenderComponent.K2_SetText` (`self.TextRender`) (`KismetTextLibrary.Conv_StringToText` (`KismetStringLibrary.TimeSecondsToString` _output_get)))
  (if (== (`self.count`) 0.0)
    (set `self.count` 3.0)
    (set `self.is potato?` false)))

(event `/Game/CookingMiniGame/GamePlay/Food/FrenchFry/Food/I_SlicePotatoFryMachine.ClickSlicePotato`
  (if (< (`self.count`) 0.0)
    _
    (elif (< (`self.count`) 1.0)
      (`|SpawnActorFromClass` "/Game/CookingMiniGame/GamePlay/Food/FrenchFry/Food/BP_FryPotato.BP_FryPotato_C" (`SceneComponent.K2_GetComponentToWorld` (`self.Scene`)) "Undefined" "MultiplyWithRoot" null null)
      (`self.K2_DestroyActor` (`self.As BP Slice Potato`)))))

(fn `UserConstructionScript`)