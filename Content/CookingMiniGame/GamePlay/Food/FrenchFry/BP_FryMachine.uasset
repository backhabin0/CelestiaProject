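; Fryer station for the cooking minigame that turns a clickable potato into a fried potato actor.
; Clicking the potato sets a busy flag, moves it, then after a delay hides it and spawns BP_FryPotato at the Scene component.
; The GetPotato event restores the potato there after a short delay and clears the flag.
; Mouse-over events are enabled at BeginPlay so hovering applies a highlight overlay material.
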(event `self.ReceiveBeginPlay`
  (set `PlayerController.bEnableMouseOverEvents` true (`GameplayStatics.GetPlayerController` 0)))

(event `self.potato.OnClicked`
  (params (TouchedComponent :type "PrimitiveComponent Object Reference") (ButtonPressed :type "Key Structure"))
  (if (not (`self.frypotato?`))
    (set `self.frypotato?` true)
    (`KismetSystemLibrary.MoveComponentTo` (`self.potato`) (0.0 0.0 -1.0) (struct) false false 0.1)
    (`KismetSystemLibrary.Delay` 3.0)
    (`SceneComponent.SetHiddenInGame` (`self.potato`) true false)
    (`|SpawnActorFromClass` "/Game/CookingMiniGame/GamePlay/Food/FrenchFry/BP_FryPotato.BP_FryPotato_C" (`SceneComponent.K2_GetComponentToWorld` (`self.Scene`)) "Undefined" "MultiplyWithRoot" null null)))

(event `self.potato.OnBeginCursorOver`
  (params (TouchedComponent :type "PrimitiveComponent Object Reference"))
  (`MeshComponent.SetOverlayMaterial` (`self.potato`) "/Game/CookingMiniGame/GamePlay/Material/M_Highlight.M_Highlight"))

(event `self.potato.OnEndCursorOver`
  (params (TouchedComponent :type "PrimitiveComponent Object Reference"))
  (`MeshComponent.SetOverlayMaterial` (`self.potato`) null))

(event `/Game/CookingMiniGame/GamePlay/Food/FrenchFry/setrepotato.getPotato`
  (bind _potato (`self.potato`))
  (`KismetSystemLibrary.Delay` 1.0)
  (`SceneComponent.K2_SetWorldLocation` _potato (`SceneComponent.K2_GetComponentLocation` (`self.Scene`)) false false)
  (`SceneComponent.SetHiddenInGame` _potato false false)
  (set `self.frypotato?` false))

(fn `UserConstructionScript`)