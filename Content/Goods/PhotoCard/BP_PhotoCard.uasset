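; BP_PhotoCard is a clickable photo card goods actor whose picture can be swapped at runtime.
; PhotoCardChange creates a dynamic material instance on the mesh and sets its Picture texture parameter.
; Cursor hover toggles a highlight overlay material.
; Clicking calls GrabFoodMessage on the cached BP_MainCharacter, passing CokeSocket and the SM_SM_GoodsCake mesh, then disables the card's collision.
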(event `self.ReceiveBeginPlay`
  (set `PlayerController.bEnableMouseOverEvents` true (`GameplayStatics.GetPlayerController` 0))
  (bind _asbp_main_character (cast `/Game/MainCharacter/BP_MainCharacter` (`GameplayStatics.GetPlayerCharacter` 0)))
  (set `self.As BP Main Character` _asbp_main_character))

(event `self.ReceiveTick`
  (params (DeltaSeconds :type "Float (single-precision)")))

(event `/Game/Goods/PhotoCard/I_PhotoCard.PhotoCardChange`
  (params (Texture :type "Texture2D Object Reference"))
  (bind _staticmesh (`self.StaticMesh`))
  (bind _returnvalue (`PrimitiveComponent.CreateDynamicMaterialInstance` _staticmesh 0 (`PrimitiveComponent.GetMaterial` _staticmesh 0) "None"))
  (`MaterialInstanceDynamic.SetTextureParameterValue` _returnvalue "Picture" Texture))

(event `self.StaticMesh.OnBeginCursorOver`
  (params (TouchedComponent :type "PrimitiveComponent Object Reference"))
  (`MeshComponent.SetOverlayMaterial` (`self.StaticMesh`) "/Game/CookingMiniGame/GamePlay/Material/M_Highlight.M_Highlight"))

(event `self.StaticMesh.OnEndCursorOver`
  (params (TouchedComponent :type "PrimitiveComponent Object Reference"))
  (`MeshComponent.SetOverlayMaterial` (`self.StaticMesh`) null))

(event `self.StaticMesh.OnClicked`
  (params (TouchedComponent :type "PrimitiveComponent Object Reference") (ButtonPressed :type "Key Structure"))
  (message `/Game/CookingMiniGame/GamePlay/I_FoodGrab.grabFood` (`self.As BP Main Character`) "CokeSocket" self "/Game/Goods/Goods/Cake/SM_SM_GoodsCake.SM_SM_GoodsCake")
  (`PrimitiveComponent.SetCollisionEnabled` (`self.StaticMesh`) "NoCollision"))

(fn `UserConstructionScript`)