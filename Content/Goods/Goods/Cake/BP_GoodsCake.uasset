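; BP_GoodsCake is a cake goods actor that highlights when the mouse cursor hovers over it.
; On BeginPlay it enables mouse-over events on the player controller, caches the player's BP_MainCharacter and turns off collision on the two-layer cake component.
; Cursor-over events on that component apply and clear a highlight overlay material.
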(event `self.ReceiveBeginPlay`
  (set `PlayerController.bEnableMouseOverEvents` true (`GameplayStatics.GetPlayerController` 0))
  (bind _asbp_main_character (cast `/Game/MainCharacter/BP_MainCharacter` (`GameplayStatics.GetPlayerCharacter` 0)))
  (set `self.As BP Main Character` _asbp_main_character)
  (`PrimitiveComponent.SetCollisionEnabled` (`self.Cake_2Layer`) "NoCollision"))

(event `self.Cake_2Layer.OnBeginCursorOver`
  (params (TouchedComponent :type "PrimitiveComponent Object Reference"))
  (`MeshComponent.SetOverlayMaterial` (`self.Cake_2Layer`) "/Game/CookingMiniGame/GamePlay/Material/M_Highlight.M_Highlight"))

(event `self.Cake_2Layer.OnEndCursorOver`
  (params (TouchedComponent :type "PrimitiveComponent Object Reference"))
  (`MeshComponent.SetOverlayMaterial` (`self.Cake_2Layer`) null))

(fn `UserConstructionScript`)