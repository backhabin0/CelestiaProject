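; BP_Poster is a clickable poster goods actor that the player character can grab and whose picture can be swapped.
; Its R component shows a highlight overlay on mouse hover, using mouse-over events enabled at BeginPlay.
; A click sends GrabFoodMessage to the cached BP_MainCharacter with a socket and the goods cake mesh, then disables R's collision.
; PhotoCardChange applies a given texture through a dynamic material instance's Picture parameter.
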(event `self.ReceiveBeginPlay`
  (set `PlayerController.bEnableMouseOverEvents` true (`GameplayStatics.GetPlayerController` 0))
  (bind _asbp_main_character (cast `/Game/MainCharacter/BP_MainCharacter` (`GameplayStatics.GetPlayerCharacter` 0)))
  (set `self.As BP Main Character` _asbp_main_character))

(event `self.r.OnBeginCursorOver`
  (params (TouchedComponent :type "PrimitiveComponent Object Reference"))
  (`MeshComponent.SetOverlayMaterial` (`self.r`) "/Game/CookingMiniGame/GamePlay/Material/M_Highlight.M_Highlight"))

(event `self.r.OnEndCursorOver`
  (params (TouchedComponent :type "PrimitiveComponent Object Reference"))
  (`MeshComponent.SetOverlayMaterial` (`self.r`) null))

(event `self.r.OnClicked`
  (params (TouchedComponent :type "PrimitiveComponent Object Reference") (ButtonPressed :type "Key Structure"))
  (message `/Game/CookingMiniGame/GamePlay/I_FoodGrab.grabFood` (`self.As BP Main Character`) "CokeSocket" self "/Game/Goods/Goods/Cake/SM_SM_GoodsCake.SM_SM_GoodsCake")
  (`PrimitiveComponent.SetCollisionEnabled` (`self.r`) "NoCollision"))

(event `/Game/Goods/Custom/PhotoCard/I_PhotoCard.PhotoCardChange`
  (params (Texture :type "Texture2D Object Reference"))
  (bind _returnvalue (`PrimitiveComponent.CreateDynamicMaterialInstance` (`self.r`) 0 null "None"))
  (`MaterialInstanceDynamic.SetTextureParameterValue` _returnvalue "Picture" Texture))

(fn `UserConstructionScript`)