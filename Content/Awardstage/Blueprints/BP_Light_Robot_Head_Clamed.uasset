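; BP_Light_Robot_Head_Clamed is a moving-head stage spotlight for the award stage, with optional automated sweeping.
; The construction script aims the arms (yaw) and head (pitch), then applies color and intensity to the spotlight and an emissive dynamic material, plus volumetric beam intensity.
; When AutomatedMove is on, Tick advances per-axis counters each frame and swings both parts on sine waves around their set angles, so speed is frame-rate dependent.
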(event `self.ReceiveTick`
  (params (DeltaSeconds :type "Float (single-precision)"))
  (bind _returnvalue (+ (`self.Horizontal_Rotation_Value`) (`self.Horizontal_Rotation_Speed`)))
  (bind _returnvalue_2 (+ (`self.Vertical_Rotation_Value`) (`self.Vertical_Rotation_Speed`)))
  ;[1 1 1] Each frame performs light rotation Angle, direction
  (if (`self.Automated Move?`)
    (set `self.Vertical_Rotation_Value` _returnvalue_2)
    (`SceneComponent.K2_SetRelativeRotation` (`self.SM_Robot_Head_Arms`) (`KismetMathLibrary.MakeRotator` 0.0 0.0 (+ (* (`KismetMathLibrary.DegSin` _returnvalue_2) (/ (`self.Vertical_Rotation_Degree_Difference`) 2.0)) (* (`self.Vertical_Rotation`) -1.0))) false false)
    (set `self.Horizontal_Rotation_Value` _returnvalue)
    (`SceneComponent.K2_SetRelativeRotation` (`self.SM_Robot_Head_Head`) (`KismetMathLibrary.MakeRotator` 0.0 (+ (* (`KismetMathLibrary.DegSin` _returnvalue) (/ (`self.Horizontal_Rotation_Degree_Difference`) 2.0)) (`self.Horizontal_Rotation (Up and Down)`))) false false)))

(fn `UserConstructionScript`
  (bind _light_intensity (`self.Light_Intensity`))
  (bind _spotlight (`self.SpotLight`))
  (bind _sm_robot_head_head (`self.SM_Robot_Head_Head`))
  (bind _light_color (`self.Light_Color`))
  ;[1 1 1] Set the light rotation direction
  (`SceneComponent.K2_SetRelativeRotation` (`self.SM_Robot_Head_Arms`) (`KismetMathLibrary.MakeRotator` 0.0 0.0 (* (`self.Vertical_Rotation`) -1.0)) false false)
  (`SceneComponent.K2_AddLocalRotation` _sm_robot_head_head (`KismetMathLibrary.MakeRotator` 0.0 (`self.Horizontal_Rotation (Up and Down)`)) false false)
  ;[1 1 1] Set light material
  (bind _returnvalue (`PrimitiveComponent.CreateDynamicMaterialInstance` _sm_robot_head_head 0 "/Game/Awardstage/Material/MI_Light_Emissive_Robot_Head.MI_Light_Emissive_Robot_Head" "None"))
  (`MaterialInstanceDynamic.SetVectorParameterValue` _returnvalue "Light_Color" _light_color)
  (`MaterialInstanceDynamic.SetScalarParameterValue` _returnvalue "Light_Emissive_Intensity" (/ _light_intensity 1000.0))
  ;;[1 1 1] Set light intensity
  (`LightComponent.SetLightColor` _spotlight _light_color true)
  (`LightComponent.SetIntensity` _spotlight _light_intensity)
  (`LightComponent.SetVolumetricScatteringIntensity` _spotlight (`self.Light Beam Intensity`)))